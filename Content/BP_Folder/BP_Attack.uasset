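; BP_Attack is a Blueprint that rates an attack as strong or weak from its Strength value and shows the result as text.
; On BeginPlay it passes Strength to CaclulateAttack, a linear formula that scales the value and adds a flat bonus.
; A threshold check on the result sets the TextRender to either the StrongAttack or WeakAttack text.
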(event `self.ReceiveBeginPlay`
  (bind _damagevalue (`self.CaclulateAttack` (`self.Strength`)))
  (if (>= _damagevalue 40)
    (`TextRenderComponent.K2_SetText` (`self.TextRender`) (`self.StrongAttack`))
    (else
      (`TextRenderComponent.K2_SetText` (`self.TextRender`) (`self.WeakAttack`)))))

(fn `CaclulateAttack`
  (params (StrengthValue :type Integer))
  (returns (DamageValue :type Integer))
  (return (+ (* StrengthValue 5) 10)))

(fn `UserConstructionScript`)